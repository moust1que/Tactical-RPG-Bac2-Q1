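; BP_Rogue is the Rogue hero Blueprint, with graph logic that drives its health and XP bar widget.
; On BeginPlay it caches the HealthBar component's WBP_HealthBar, stopping if the cast fails, then binds handlers to the health and XP change events.
; It fires both events with hardcoded starting values, and the handlers forward every change to the widget's update functions.
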(event `self.ReceiveBeginPlay`
  (bind _aswbp_health_bar (cast `/Game/Blueprint/Widgets/WBP_HealthBar` (`WidgetComponent.GetUserWidgetObject` (`self.HealthBar`))))
  (set `self.WBP Health Bar` _aswbp_health_bar)
  (add `self.OnHealthChanged` (delegate `OnHealthChanged_Event`))
  (`self.OnHealthChanged_Event` 80.0 80.0)
  (add `self.OnXPChanged` (delegate `OnXPChanged_Event`))
  (`self.OnXPChanged_Event` 0.0 100.0))

(event `OnHealthChanged_Event` :!signature `self.OnHealthChanged`
  (params (Health :type "Float (single-precision)") (MaxHealth :type "Float (single-precision)"))
  (`/Game/Blueprint/Widgets/WBP_HealthBar.UpdateHealthBar` (`self.WBP Health Bar`) Health MaxHealth))

(event `OnXPChanged_Event` :!signature `self.OnXPChanged`
  (params (XP :type "Float (single-precision)") (XPForNextLevel :type "Float (single-precision)"))
  (`/Game/Blueprint/Widgets/WBP_HealthBar.UpdateXPBar` (`self.WBP Health Bar`) XP XPForNextLevel))

(fn `UserConstructionScript`)